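; BP_Cube is a breakable cube that reacts to hits from BP_Ball and drops a random actor when it breaks.
; While HP is above zero, each ball hit applies the damaged material and decrements HP.
; A hit at zero HP spawns a random entry from the Class array at the cube's location, then destroys the hit component rather than the actor.
; The weighted drop roll is set to always pass.
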(event EventBeginPlay)

(event Collision|EventActorBeginOverlap
  (params (OtherActor :type Actor%20Object%20Reference)))

(event EventTick
  (params (DeltaSeconds :type Float%20%28single-precision%29)))

(event Collision|EventHit
  (params (MyComp :type Primitive%20Component%20Object%20Reference) (Other :type Actor%20Object%20Reference) (OtherComp :type Primitive%20Component%20Object%20Reference) (bSelfMoved :type Boolean) (HitLocation :type Vector :default "0, 0, 0") (HitNormal :type Vector :default "0, 0, 0") (NormalImpulse :type Vector :default "0, 0, 0") (Hit :type Hit%20Result%20Structure%20%28by%20ref%29))
  (bind _class (Variables|Default|GetClass))
  (Utilities|Casting|CastToBP_Ball Other)
  (if (> (Variables|Default|GetHP) 0)
    (Rendering|Material|SetMaterial (Variables|Default|GetCube) 0 "/Game/Materials/M_DamageCubeColor.M_DamageCubeColor")
    (bind _result (Math|Integer|DecrementInt (Variables|Default|GetHP))
      (:%20%20
        (Variables|Default|SetHP _result)))
    (elif (Math|Random|RandomBoolwithWeight 1.0)
      (Game|SpawnActorfromClass (Utilities|Array|Get(acopy) _class (Math|Random|RandomInteger (Utilities|Array|Length _class))) (Math|Transform|MakeTransform (Transformation|GetWorldLocation (Variables|Default|GetCube)) "0, 0, 0" "1,1,1") "AlwaysSpawn" 0 0)
      (Components|DestroyComponent MyComp))))

(fn ConstructionScript)