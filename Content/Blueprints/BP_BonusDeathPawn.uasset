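; BP_BonusDeathPawn is a death pickup that kills any BP_Pawn that touches it.
; On actor overlap it calls the parent handler, casts the other actor to BP_Pawn, then destroys itself and that pawn and prints a long-lasting on-screen death message.
; Other actors are ignored after the parent call, BeginPlay and Tick are disabled, and the construction script only calls its parent.
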(event EventBeginPlay
  (|CallParentFunction) ; This node is disabled and will not be called.\nDrag off pins to build functionality.
)

(event Collision|EventActorBeginOverlap
  (params (OtherActor :type Actor%20Object%20Reference))
  (|CallParentFunction OtherActor)
  (bind _asbp_pawn (Utilities|Casting|CastToBP_Pawn OtherActor))
  (Actor|DestroyActor)
  (Actor|DestroyActor _asbp_pawn)
  (Development|PrintString "Pawn is death" true true "(R=0.000000,G=0.000000,B=0.000000,A=1.000000)" 6e+01))

(event EventTick
  (params (DeltaSeconds :type Float%20%28single-precision%29))
  (|CallParentFunction DeltaSeconds) ; This node is disabled and will not be called.\nDrag off pins to build functionality.
)

(fn ConstructionScript
  (|CallParentFunction))