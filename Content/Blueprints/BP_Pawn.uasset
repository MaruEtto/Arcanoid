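; BP_Pawn is a player pawn that slides left and right and spawns the ball in play, apparently a paddle.
; Two MoveRight axis handlers move it along world Y by a fixed swept step, using only the input's sign without delta-time scaling.
; On BeginPlay, SpawnBall creates a BP_Ball at the capsule's location, stores it as PlayingBall and binds to its OnDead event.
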(event EventBeginPlay
  ;[1 1 1] Создание шарика
  (CallFunction|SpawnBall))

(event Collision|EventActorBeginOverlap
  (params (OtherActor :type Actor%20Object%20Reference)))

(event EventTick
  (params (DeltaSeconds :type Float%20%28single-precision%29)))

(event Input|AxisEvents|InputAxisMoveRight
  (params (AxisValue :type Float%20%28single-precision%29))
  ;[1 1 1] Движение влево
  (if (< AxisValue 0.0)
    (Transformation|AddActorWorldOffset "0,-40.000000, 0" true)))

(event Input|AxisEvents|InputAxisMoveRight
  (params (AxisValue :type Float%20%28single-precision%29))
  ;[1 1 1] Движение вправо
  (if (> AxisValue 0.0)
    (Transformation|AddActorWorldOffset "0,40.000000, 0" true)))

(fn ConstructionScript)

(fn SpawnBall
  (bind _returnvalue (Game|SpawnActorfromClass "/Game/Blueprints/BP_Ball.BP_Ball_C" (Math|Transform|MakeTransform (Transformation|GetWorldLocation (Variables|Default|GetCapsule)) "0, 0, 0" "1,1,1") "AlwaysSpawn" 0 0))
  (bind _output_get (Variables|Default|SetPlayingBall _returnvalue))
  (EventDispatchers|BindEventtoOnDead _output_get (EventDispatchers|CreateEvent :!event SpawnBall))
  (return))